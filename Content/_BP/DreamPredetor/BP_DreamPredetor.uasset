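; BP_DreamPredetor is a character Blueprint for a predator that stops moving while it attacks.
; It applies MoveSpeed as walk speed on BeginPlay, and StartAttack, guarded by a DoOnce, zeroes that speed and sets CanAttack.
; EndAttack resets the DoOnce, restores MoveSpeed, clears CanAttack and sets IsEndAttack.
; The attack events only change movement and state flags, with no damage or targeting logic in these graphs.
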(event Custom|Start%20Attack
  (Utilities|FlowControl|DoOnce false
    (:Completed
      (Variables|/Script/Engine.CharacterMovementComponent|SetMaxWalkSpeed (Variables|Character|GetCharacterMovement) 0.0)
      (Variables|Default|SetCanAttack true))))

(event Custom|End%20Attack
  (Utilities|FlowControl|Sequence
    (:then_0
      (Utilities|FlowControl|DoOnce false) ; enters at Reset
    )
    (:then_1
      (Variables|/Script/Engine.CharacterMovementComponent|SetMaxWalkSpeed (Variables|Character|GetCharacterMovement) (Variables|Default|GetMoveSpeed))
      (Variables|Default|SetCanAttack false)
      (Variables|Default|SetIsEndAttack true))))

(event EventBeginPlay
  (Variables|/Script/Engine.CharacterMovementComponent|SetMaxWalkSpeed (Variables|Character|GetCharacterMovement) (Variables|Default|GetMoveSpeed)))

(event Collision|EventActorBeginOverlap
  (params (OtherActor :type Actor%20Object%20Reference)))

(event EventTick
  (params (DeltaSeconds :type Float%20%28single-precision%29)))

(fn ConstructionScript)