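; BP_TutorialNpc is a tutorial NPC that shows a sequence of dialogue lines in a UI widget, then removes itself.
; TalkStart runs once through a DoOnce, advancing TalkIndex and creating a WB_Talk widget with that line from the Dialogue array.
; TalkNext steps through the remaining lines, and past the last one it removes the widget and destroys the actor.
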(event EventBeginPlay)

(event EventTalkNext
  (Math|Integer|IncrementInt (Variables|Default|GetTalk%20Index)
    (:%20%20
      (if (< (Variables|Default|GetTalk%20Index) (Utilities|Array|Length (Variables|Default|GetDialogue)))
        (Variables|Default|GetUI
          (:then
            (Rendering|Components|TextRender|SetText (Variables|/Game/_BP/UI/WB_Talk.WB_Talk_C|GetTalkText (Variables|Default|GetUI)) (Utilities|Text|ToText(String) (Utilities|Array|Get(acopy) (Variables|Default|GetDialogue) (Variables|Default|GetTalk%20Index)))))
          (:else))
        (else
          (Widget|RemovefromParent (Variables|Default|GetUI))
          (Actor|DestroyActor)
          (Variables|Default|SetTalk%20Index -1))))))

(event EventTick
  (params (DeltaSeconds :type Float%20%28single-precision%29)))

(event EventTalkStart
  (Utilities|FlowControl|DoOnce false
    (:Completed
      (Math|Integer|IncrementInt (Variables|Default|GetTalk%20Index)
        (:%20%20
          (if (< (Variables|Default|GetTalk%20Index) (Utilities|Array|Length (Variables|Default|GetDialogue)))
            (bind _returnvalue (UserInterface|CreateWidget "/Game/_BP/UI/WB_Talk.WB_Talk_C" (Game|GetPlayerController 0)))
            (bind _output_get (Variables|Default|SetUI _returnvalue))
            (UserInterface|Viewport|AddtoViewport _output_get 0)
            (Rendering|Components|TextRender|SetText (Variables|/Game/_BP/UI/WB_Talk.WB_Talk_C|GetTalkText (Variables|Default|GetUI)) (Utilities|Text|ToText(String) (Utilities|Array|Get(acopy) (Variables|Default|GetDialogue) (Variables|Default|GetTalk%20Index))))))))))

(fn ConstructionScript)