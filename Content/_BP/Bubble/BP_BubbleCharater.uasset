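; Player bubble character driven by microphone-style audio input, with a noise-cancel ability and an on-screen sound bar widget.
; AudioCapture envelope values are log-mapped to loudness, pushing the bubble backward along its local X axis; GetRotation turns it toward a supplied target.
; Holding noise cancel stops that movement and, given enough sound, sphere-traces around Arrow2, sending DeleteNoiseMessage once per actor until release.
; A debug key toggles constant test movement.
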(event OnAudioEnvelopeValue(AudioCapture)
  (params (EnvelopeValue :type Float%20%28single-precision%29))
  (bind _inputsound (Variables|Default|GetInputSound))
  ;[0.02732 0.02732 0.02732] 소리의 역방향으로 이동
  (bind _output_get (Variables|Default|SetinputSound (Math|Float|MapRangeClamped (Math|Float|Log EnvelopeValue 1e+01) -2.5 -0.5 0.0 1.0)))
  (if (< _inputsound 9.0)
    (if (not (Variables|Default|GetIsNoiseCancel))
      (Transformation|AddActorLocalOffset (Math|Vector|MakeVector (* _inputsound -1e+01) 0.0 0.0) false false))))

(event Input|EnhancedActionEvents|EnhancedInputActionIA_NoiseCancel
  (params (ActionValue :type Boolean) (ElapsedSeconds :type Float%20%28double-precision%29) (TriggeredSeconds :type Float%20%28double-precision%29) (InputAction :type Input%20Action%20Object%20Reference :default "/Game/_BP/Bubble/input/IA_NoiseCancel.IA_NoiseCancel"))
  (bind _arrow2 (Variables|Default|GetArrow2))
  (bind _returnvalue (Transformation|GetWorldLocation _arrow2))
  ;[0.02732 0.02732 0.02732] 노이즈 캔슬링
  (:Triggered
    ;;[0.02732 0.02732 0.02732] 노이즈 캔슬링범위
    (if (> (Variables|Default|GetinputSound) 0.1)
      (bind _outhits (Collision|MultiSphereTraceByChannel _returnvalue _returnvalue 3e+02 "TraceTypeQuery1" false 0 "ForDuration" true "(R=1.000000,G=0.000000,B=0.000000,A=1.000000)" "(R=0.000000,G=1.000000,B=0.000000,A=1.000000)" 0.1))
      (bind _output_get (Variables|Default|SetOut%20Hits _outhits))
      (for _array_element _output_get
        (Utilities|IsValid (.hitactor _array_element)
          (:Is%20Valid
            (bind _canhit (CallFunction|CanHit? (.hitactor _array_element)))
            (if _canhit
              (Development|PrintString (Utilities|GetDisplayName (.hitactor _array_element)))
              (Class|OverlapNoise|DeleteNoise(Message) (.hitactor _array_element))
              (Utilities|Array|Add (Variables|Default|GetHit%20Actor%20Array) (.hitactor _array_element))))))))
  (:Started
    ;;[0.02732 0.02732 0.02732] 노이즈 캔슬링 시작
    (if (not (Variables|Default|GetIsNoiseCancel))
      (Variables|Default|SetIsNoiseCancel true)
      (Development|PrintString "on")))
  (:Canceled
    ;;[0.02732 0.02732 0.02732] 노이즈 캔슬링 종료
    (Variables|Default|SetIsNoiseCancel false :!label _label)
    (Development|PrintString "off")
    (Utilities|Array|Clear (Variables|Default|GetHit%20Actor%20Array)))
  (:Completed
    (goto _label)))

(event EventBeginPlay
  ;[0.02732 0.02732 0.02732] 사운드바 출력
  (bind _as플레이어_컨트롤러 (Utilities|Casting|CastToPlayerController (Pawn|GetController)))
  (Utilities|IsValid (PlayerController|LocalPlayerSubsystems|GetEnhancedInputLocalPlayerSubsystem _as플레이어_컨트롤러)
    (:Is%20Valid
      (Input|AddMappingContext (PlayerController|LocalPlayerSubsystems|GetEnhancedInputLocalPlayerSubsystem _as플레이어_컨트롤러) "/Game/_BP/Bubble/input/InputMappingContext.InputMappingContext" 0 "(bIgnoreAllPressedKeysUntilRelease=True,bForceImmediately=False,bNotifyUserSettings=False)")
      (bind _returnvalue (UserInterface|CreateWidget "/Game/_BP/UI/WB_SoundBar.WB_SoundBar_C"))
      (UserInterface|Viewport|AddtoViewport _returnvalue 0))))

(event EventTick
  (params (DeltaSeconds :type Float%20%28single-precision%29))
  (if (Variables|Default|GetDebug%20On)
    (bind _output_get (Variables|Default|SetinputSound -2.0))
    (Development|PrintString "Debuging")
    (Transformation|AddActorLocalOffset (Math|Vector|MakeVector _output_get 0.0 0.0) false false)))

(event EventHitNoise
  (Variables|Default|SetCan%20Move false)
  (Development|PrintString "Hit"))

(event EventGetRotation
  (params (targetVector :type Vector :default "0, 0, 0"))
  (bind _returnvalue (Transformation|GetActorLocation))
  ;[0.02732 0.02732 0.02732] 버블회전
  (bind _output_get (Variables|Default|SetMouse%20Vector targetVector))
  (Transformation|SetActorRotation (Math|Rotator|FindLookatRotation (Math|Vector|MakeVector (.x _returnvalue) (.y _returnvalue) 0.0) (Math|Vector|MakeVector (.x _output_get) (.y _output_get) 0.0))))

(event Input|KeyboardEvents|DebugKeySpaceBar
  (params (Key :type Key%20Structure :default "None") (ActionValue :type Input%20Action%20Value%20Structure))
  (:Pressed
    (Development|PrintString "Hello")
    (if (Variables|Default|GetDebug%20On)
      (Variables|Default|SetDebug%20On false)
      (Development|PrintString "Debug Off")
      (else
        (Variables|Default|SetDebug%20On true)
        (Development|PrintString "Debug On")))))

(fn ConstructionScript)

(fn CanHit?
  (params (Hit%20Actor :type Object%20Object%20Reference))
  (for _array_element (Variables|Default|GetHit%20Actor%20Array)
    (if (== _array_element Hit%20Actor)
      (return false)))
  (return true))